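; BP_HealthPack is a health pickup that heals the player on overlap.
; When a BP_Player with Health below 1.0 overlaps it, it adds a fixed amount without clamping and destroys itself.
; At full health the pack stays in place.
; RandomizeHealthPack applies a local offset of X/Y/Z plus random per-axis jitter within the Xrand/Yrand/Zrand ranges, but nothing in this Blueprint calls it.
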(event `self.ReceiveActorBeginOverlap`
  (params (OtherActor :type "Actor Object Reference"))
  (bind _asbp_player (cast `/Game/InfiniteMatrix/Blueprints/BP_Player` OtherActor))
  (bind _health (`/Game/InfiniteMatrix/Blueprints/BP_Player.Health` _asbp_player))
  (if (< _health 1.0)
    (set `/Game/InfiniteMatrix/Blueprints/BP_Player.Health` (+ _health 0.15) _asbp_player)
    (`self.K2_DestroyActor`)))

(fn `RandomizeHealthPack`
  (bind _xrand (`self.Xrand`))
  (bind _zrand (`self.Zrand`))
  (bind _yrand (`self.Yrand`))
  (`self.K2_AddActorLocalTransform` (`KismetMathLibrary.MakeTransform` (`KismetMathLibrary.MakeVector` (+ (`self.X`) (`KismetMathLibrary.RandomFloatInRange` (* _xrand -1.0) _xrand)) (+ (`self.Y`) (`KismetMathLibrary.RandomFloatInRange` (* _yrand -1.0) _yrand)) (+ (`self.Z`) (`KismetMathLibrary.RandomFloatInRange` (* _zrand -1.0) _zrand))))))

(fn `UserConstructionScript`)