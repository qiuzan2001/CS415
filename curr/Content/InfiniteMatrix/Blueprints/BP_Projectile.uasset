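; BP_Projectile is a bullet that destroys enemies and rewards the player for each kill.
; Tick moves it along world X at BulletSpeed using a swept offset.
; Any overlap destroys the projectile; if the other actor is a BP_Enemy, it calls Rewards and destroys that enemy.
; Rewards raises Score and lowers ForwardSpeed on the BPplayer reference, which is not assigned in these graphs.
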(event `self.ReceiveActorBeginOverlap`
  (params (OtherActor :type "Actor Object Reference"))
  (`self.K2_DestroyActor`)
  (bind _asbp_enemy (cast `/Game/InfiniteMatrix/Blueprints/BP_Enemy` OtherActor))
  (`self.Rewards`)
  (`self.K2_DestroyActor` _asbp_enemy))

(event `self.ReceiveTick`
  (params (DeltaSeconds :type "Float (single-precision)"))
  (`self.K2_AddActorWorldOffset` (`KismetMathLibrary.MakeVector` (* DeltaSeconds (`self.BulletSpeed`))) true))

(fn `Rewards`
  (bind _bpplayer (`self.BPplayer`))
  (set `/Game/InfiniteMatrix/Blueprints/BP_Player.Score` (+ (`/Game/InfiniteMatrix/Blueprints/BP_Player.Score` _bpplayer) 100.0) _bpplayer)
  (set `/Game/InfiniteMatrix/Blueprints/BP_Player.ForwardSpeed` (- (`/Game/InfiniteMatrix/Blueprints/BP_Player.ForwardSpeed` _bpplayer) 500.0) _bpplayer))

(fn `UserConstructionScript`)