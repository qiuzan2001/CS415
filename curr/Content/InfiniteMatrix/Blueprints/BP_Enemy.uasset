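; BP_Enemy is an enemy actor that damages BP_Player on overlap.
; On contact it plays a world camera shake at the player, with outer radius scaled by forward speed, reduces health and destroys itself.
; When health runs out, it flags the player dead and displays the restart.
; RandomizeEnemy, not called within this Blueprint, offsets the actor's local position randomly within per-axis ranges.
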(event `self.ReceiveActorBeginOverlap`
  (params (OtherActor :type "Actor Object Reference"))
  (bind _asbp_player (cast `/Game/InfiniteMatrix/Blueprints/BP_Player` OtherActor))
  (`self.shake` _asbp_player)
  (bind _output_get (set `/Game/InfiniteMatrix/Blueprints/BP_Player.Health` (- (`/Game/InfiniteMatrix/Blueprints/BP_Player.Health` _asbp_player) 0.1) _asbp_player))
  (`self.K2_DestroyActor`)
  (if (<= _output_get 0.0)
    (set `/Game/InfiniteMatrix/Blueprints/BP_Player.IsDead` true _asbp_player)
    (`/Game/InfiniteMatrix/Blueprints/BP_Player.DisplayRestart` _asbp_player)))

(fn `RandomizeEnemy`
  (bind _xrand (`self.Xrand`))
  (bind _zrand (`self.Zrand`))
  (bind _yrand (`self.Yrand`))
  (`self.K2_AddActorLocalTransform` (`KismetMathLibrary.MakeTransform` (`KismetMathLibrary.MakeVector` (+ (`self.X`) (`KismetMathLibrary.RandomFloatInRange` (* _xrand -1.0) _xrand)) (+ (`self.Y`) (`KismetMathLibrary.RandomFloatInRange` (* _yrand -1.0) _yrand)) (+ (`self.Z`) (`KismetMathLibrary.RandomFloatInRange` (* _zrand -1.0) _zrand))))))

(fn `shake`
  (params (BPPlayer :type "/Game/InfiniteMatrix/Blueprints/BP_Player Object Reference"))
  (`GameplayStatics.PlayWorldCameraShake` "/Game/InfiniteMatrix/Blueprints/BP_Shake.BP_Shake_C" (`self.K2_GetActorLocation` BPPlayer) 0.0 (* (`/Game/InfiniteMatrix/Blueprints/BP_Player.ForwardSpeed` BPPlayer) 0.1))
  (return))

(fn `UserConstructionScript`)